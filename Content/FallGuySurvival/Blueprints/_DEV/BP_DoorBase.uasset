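; BP_DoorBase is an interactable door that toggles between open and closed.
; Each Interact flips IsOpen, then plays or reverses the DoorRotationLeft timeline, whose ZRotation track sets the relative yaw of DoorLeft.
; It always reports itself as interactable and supplies "Close" or "Open" as interaction text based on IsOpen.
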(event `InteractionInterface.Interact`
  (params (Caller :type "TFCharacter Object Reference"))
  (bind _output_get (set `self.bIsOpen` (not (`self.bIsOpen`))))
  (if _output_get
    (bind (_direction _zrotation) (`Timeline|DoorRotationLeft` :!label _label)
      (:`Update`
        (`SceneComponent.K2_SetRelativeRotation` (`self.DoorLeft`) (`KismetMathLibrary.MakeRotator` 0.0 0.0 _zrotation) false false)))
    (else
      (goto _label :!via `Reverse`))))

(fn `GetInteractionText`
  (returns (ReturnValue :type Text))
  (return (`KismetMathLibrary.SelectText` "Close" "Open" (`self.bIsOpen`))))

(fn `IsInteractable`
  (returns (ReturnValue :type Boolean))
  (return true))

(fn `UserConstructionScript`)