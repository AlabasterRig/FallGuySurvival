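; A development test Blueprint for a building door that swings open and closed when interacted with.
; Interact toggles IsOpen and plays or reverses a timeline that drives the door's relative yaw.
; When the timeline finishes, the parent building recalculates its seal.
; UpdatefromSave snaps the door straight to its open or closed rotation based on IsOpen.
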(event `InteractionInterface.Interact`
  (params (Caller :type "TFCharacter Object Reference"))
  (bind _output_get (set `self.bIsOpen` (not (`self.bIsOpen`))))
  (if _output_get
    (bind (_direction _doorleft) (`Timeline|Timeline` :!label _label)
      (:`Update`
        (`SceneComponent.K2_SetRelativeRotation` (`self.Door`) (`KismetMathLibrary.MakeRotator` 0.0 0.0 _doorleft) false false))
      (:`Finished`
        (`TFBuildingBase.RecalculateSeal` (`self.ParentBuilding`))))
    (else
      (goto _label :!via `Reverse`))))

(event `SaveActorInterface.UpdateFromSave`
  (`SceneComponent.K2_SetRelativeRotation` (`self.Door`) (`KismetMathLibrary.MakeRotator` 0.0 0.0 (`KismetMathLibrary.SelectFloat` 110.0 0.0 (`self.bIsOpen`))) false false))

(fn `UserConstructionScript`)