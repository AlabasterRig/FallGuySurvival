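; Development base Blueprint for an interactable double door that toggles open and closed, with an Open or Close prompt that follows its state.
; Interact flips IsOpen and plays or reverses the DoorRotation timeline, whose two tracks drive the yaw of the left and right leaves.
; UpdatefromSave skips the animation and snaps both leaves to mirrored open or closed angles based on IsOpen.
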(event `InteractionInterface.Interact`
  (params (Caller :type "TFCharacter Object Reference"))
  (bind _output_get (set `self.bIsOpen` (not (`self.bIsOpen`))))
  (if _output_get
    (bind (_direction _doorleft _doorright) (`Timeline|DoorRotation` :!label _label)
      (:`Update`
        (`SceneComponent.K2_SetRelativeRotation` (`self.DoorLeft`) (`KismetMathLibrary.MakeRotator` 0.0 0.0 _doorleft) false false)
        (`SceneComponent.K2_SetRelativeRotation` (`self.DoorRight`) (`KismetMathLibrary.MakeRotator` 0.0 0.0 _doorright) false false)))
    (else
      (goto _label :!via `Reverse`))))

(event `SaveActorInterface.UpdateFromSave`
  (bind _returnvalue (`KismetMathLibrary.SelectFloat` 110.0 0.0 (`self.bIsOpen`)))
  (`SceneComponent.K2_SetRelativeRotation` (`self.DoorLeft`) (`KismetMathLibrary.MakeRotator` 0.0 0.0 _returnvalue) false false)
  (`SceneComponent.K2_SetRelativeRotation` (`self.DoorRight`) (`KismetMathLibrary.MakeRotator` 0.0 0.0 (* _returnvalue -1.0)) false false))

(fn `GetInteractionText`
  (returns (ReturnValue :type Text))
  (return (`KismetMathLibrary.SelectText` "Close" "Open" (`self.bIsOpen`))))

(fn `IsInteractable`
  (returns (ReturnValue :type Boolean))
  (return true))

(fn `UserConstructionScript`)