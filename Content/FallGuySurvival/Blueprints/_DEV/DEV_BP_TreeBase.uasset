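; Development base Blueprint for a harvestable tree with a main mesh, a stump mesh and a collision capsule.
; Any overlap with the capsule makes the tree take fixed damage, with the overlapping actor as causer.
; The harvested event prints a debug message and destroys the capsule and main mesh.
; Nodes that would reveal the stump are unconnected and never run.
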(event `self.Capsule.OnComponentBeginOverlap`
  (params (OverlappedComponent :type "PrimitiveComponent Object Reference") (OtherActor :type "Actor Object Reference") (OtherComp :type "PrimitiveComponent Object Reference") (OtherBodyIndex :type Integer) (bFromSweep :type Boolean) (SweepResult :type "HitResult Structure (by ref)"))
  (`self.TakeDamage` 50.0 (make `DamageEvent`) null OtherActor))

(event `self.OnHarvestedBP`
  (`KismetSystemLibrary.PrintString` "Harvested")
  (`ActorComponent.K2_DestroyComponent` (`self.Capsule`))
  (`ActorComponent.K2_DestroyComponent` (`self.MainTreeMesh`)))

(fn `UserConstructionScript`)